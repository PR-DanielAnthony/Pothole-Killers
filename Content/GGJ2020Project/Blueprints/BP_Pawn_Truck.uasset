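; Player truck pawn for a lane-based shooter that hops between preset move spots and fires projectiles.
; It starts at the center spot, and Up/Down input teleports it to the adjacent spot, whose links become its new neighbors.
; Shoot spawns a BP_Actor_Projectile that references the pawn.
; UpdateScore clamps the score at zero, refreshes the HUD text and, at score milestones, retunes every spawner's timing and index ranges.
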(event `self.ReceiveBeginPlay`
  (bind _movespotcenter (`self.MoveSpotCenter`)
    (:`then`
      (`self.K2_TeleportTo` (`self.K2_GetActorLocation` _movespotcenter) (`self.K2_GetActorRotation`)))
    (:`else`)))

(event `InputAction|MoveUp`
  (params (Key :type "Key Structure"))
  (:`Pressed`
    (bind _movespotup (`self.MoveSpotUp`)
      (:`then`
        (bind _returnvalue (`self.K2_TeleportTo` (`self.K2_GetActorLocation` _movespotup) (`self.K2_GetActorRotation`)))
        (if _returnvalue
          (set `self.MoveSpotDown` (`/Game/GGJ2020Project/Blueprints/BP_Actor_MoveSpot.MoveSpotDown` _movespotup))
          (set `self.MoveSpotUp` (`/Game/GGJ2020Project/Blueprints/BP_Actor_MoveSpot.MoveSpotUp` _movespotup))))
      (:`else`))))

(event `InputAction|MoveDown`
  (params (Key :type "Key Structure"))
  (:`Pressed`
    (bind _movespotdown (`self.MoveSpotDown`)
      (:`then`
        (bind _returnvalue (`self.K2_TeleportTo` (`self.K2_GetActorLocation` _movespotdown) (`self.K2_GetActorRotation`)))
        (if _returnvalue
          (set `self.MoveSpotUp` (`/Game/GGJ2020Project/Blueprints/BP_Actor_MoveSpot.MoveSpotUp` _movespotdown))
          (set `self.MoveSpotDown` (`/Game/GGJ2020Project/Blueprints/BP_Actor_MoveSpot.MoveSpotDown` _movespotdown))))
      (:`else`))))

(event `InputAction|Shoot`
  (params (Key :type "Key Structure"))
  (:`Pressed`
    (`|SpawnActorFromClass` "/Game/GGJ2020Project/Blueprints/BP_Actor_Projectile.BP_Actor_Projectile_C" (`self.GetTransform`) "AlwaysSpawn" "OverrideRootScale" null self null)))

(fn `UpdateScore`
  (params (Score :type Integer))
  (bind _returnvalue (+ Score (`self.Score`)))
  (if (<= _returnvalue 0)
    (set `self.Score` 0)
    (else
      (set `self.Score` _returnvalue)))
  (`TextBlock.SetText` (`/Game/GGJ2020Project/Widgets/WB_Main.ScoreText` (`self.WB_Main`)) (`|FormatText` "SCORE - {Score} pts" (`KismetTextLibrary.Conv_IntToText` (`self.Score`) false false)))
  (if (>= (`self.Score`) 5000)
    (if (>= (`self.Score`) 15000)
      (if (>= (`self.Score`) 30000)
        (bind _outactors (`GameplayStatics.GetAllActorsOfClass` "/Game/GGJ2020Project/Blueprints/BP_Actor_Spawner.BP_Actor_Spawner_C"))
        (for _array_element _outactors
          (set `/Game/GGJ2020Project/Blueprints/BP_Actor_Spawner.MinTime` 0.5 _array_element)
          (set `/Game/GGJ2020Project/Blueprints/BP_Actor_Spawner.MaxTime` 1.0 _array_element)
          (set `/Game/GGJ2020Project/Blueprints/BP_Actor_Spawner.MinIndex` 3 _array_element)
          (set `/Game/GGJ2020Project/Blueprints/BP_Actor_Spawner.MaxIndex` 8 _array_element))
        (return)
        (else
          (bind _outactors_2 (`GameplayStatics.GetAllActorsOfClass` "/Game/GGJ2020Project/Blueprints/BP_Actor_Spawner.BP_Actor_Spawner_C"))
          (for _array_element_2 _outactors_2
            (set `/Game/GGJ2020Project/Blueprints/BP_Actor_Spawner.MinTime` 1.0 _array_element_2)
            (set `/Game/GGJ2020Project/Blueprints/BP_Actor_Spawner.MaxTime` 2.0 _array_element_2)
            (set `/Game/GGJ2020Project/Blueprints/BP_Actor_Spawner.MinIndex` 2 _array_element_2)
            (set `/Game/GGJ2020Project/Blueprints/BP_Actor_Spawner.MaxIndex` 7 _array_element_2))
          (return)))
      (else
        (bind _outactors_3 (`GameplayStatics.GetAllActorsOfClass` "/Game/GGJ2020Project/Blueprints/BP_Actor_Spawner.BP_Actor_Spawner_C"))
        (for _array_element_3 _outactors_3
          (set `/Game/GGJ2020Project/Blueprints/BP_Actor_Spawner.MinTime` 2.0 _array_element_3)
          (set `/Game/GGJ2020Project/Blueprints/BP_Actor_Spawner.MaxTime` 4.0 _array_element_3)
          (set `/Game/GGJ2020Project/Blueprints/BP_Actor_Spawner.MinIndex` 1 _array_element_3)
          (set `/Game/GGJ2020Project/Blueprints/BP_Actor_Spawner.MaxIndex` 6 _array_element_3))
        (return)))))

(fn `UserConstructionScript`)