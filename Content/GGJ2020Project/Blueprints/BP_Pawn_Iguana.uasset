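; BP_Pawn_Iguana is an iguana pawn that travels steadily along the negative world Y axis.
; On BeginPlay it plays a sound at its location with a slightly randomized, raised pitch.
; Tick offsets the actor by Speed scaled by delta time, without sweeping for collisions.
; DecreaseSpeed halves Speed but clamps it to a minimum, so the iguana never stops.
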(event `self.ReceiveBeginPlay`
  (`GameplayStatics.PlaySoundAtLocation` null (`self.K2_GetActorLocation`) (struct) 2.0 (`KismetMathLibrary.RandomFloatInRange` 1.0 1.5) 0.0 null null null))

(event `self.ReceiveTick`
  (params (DeltaSeconds :type "Float (single-precision)"))
  (`self.K2_AddActorWorldOffset` (`KismetMathLibrary.MakeVector` 0.0 (* DeltaSeconds (`self.Speed`) -1.0))))

(fn `DecreaseSpeed`
  (set `self.Speed` (/ (`self.Speed`) 2.0))
  (if (<= (`self.Speed`) 100.0)
    (set `self.Speed` 100.0)
    (return)
    (else
      (return))))

(fn `UserConstructionScript`)