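; BP_Actor_Pothole is a road hazard that penalizes the player's score when driven over.
; Each Tick it moves along negative world Y at Speed, without sweeping.
; Its Box overlap costs BP_Pawn_Truck points and plays a bump sound.
; A BP_Pawn_Car hit instead slows that car, adds randomly pitched cursing to the bump, and docks the player truck a larger penalty.
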(event `self.ReceiveTick`
  (params (DeltaSeconds :type "Float (single-precision)"))
  (`self.K2_AddActorWorldOffset` (`KismetMathLibrary.MakeVector` 0.0 (* DeltaSeconds (`self.Speed`) -1.0))))

(event `self.Box.OnComponentBeginOverlap`
  (params (OverlappedComponent :type "PrimitiveComponent Object Reference") (OtherActor :type "Actor Object Reference") (OtherComp :type "PrimitiveComponent Object Reference") (OtherBodyIndex :type Integer) (bFromSweep :type Boolean) (SweepResult :type "HitResult Structure (by ref)"))
  (bind _returnvalue (`self.K2_GetActorLocation`))
  (bind _asbp_pawn_truck (cast `/Game/GGJ2020Project/Blueprints/BP_Pawn_Truck` OtherActor)
    (:`then`
      (`/Game/GGJ2020Project/Blueprints/BP_Pawn_Truck.UpdateScore` _asbp_pawn_truck -1000)
      (`GameplayStatics.PlaySoundAtLocation` "/Game/GGJ2020Project/Sounds/SW_CarPotholeBump.SW_CarPotholeBump" (`self.K2_GetActorLocation`) (struct) 3.0 1.0 0.0 null null null))
    (:`CastFailed`
      (bind _asbp_pawn_car (cast `/Game/GGJ2020Project/Blueprints/BP_Pawn_Car` OtherActor))
      (`/Game/GGJ2020Project/Blueprints/BP_Pawn_Car.DecreaseSpeed` _asbp_pawn_car)
      (`GameplayStatics.PlaySoundAtLocation` "/Game/GGJ2020Project/Sounds/SW_CarPotholeBump.SW_CarPotholeBump" _returnvalue (struct) 3.0 1.0 0.0 null null null)
      (`GameplayStatics.PlaySoundAtLocation` "/Game/GGJ2020Project/Sounds/SW_CursingGibberish.SW_CursingGibberish" _returnvalue (struct) 3.0 (`KismetMathLibrary.RandomFloatInRange` 1.0 1.5) 0.0 null null null)
      (`/Game/GGJ2020Project/Blueprints/BP_Pawn_Truck.UpdateScore` (cast `/Game/GGJ2020Project/Blueprints/BP_Pawn_Truck` (`GameplayStatics.GetPlayerPawn` 0) :!pure true) -2000))))

(fn `UserConstructionScript`)