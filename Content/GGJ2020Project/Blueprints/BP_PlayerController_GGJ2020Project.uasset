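; Player controller for the GGJ2020 truck game, handling HUD setup, music and the game-over flow.
; On BeginPlay it caches the truck pawn, creates and shares the main widget, starts audio and switches to unlit view via console command.
; GameOver shows the final score, halts cars, potholes and background scroll, destroys spawners, disables truck input and swaps the sound.
; The MoveMenu input then moves from game over to scrolling credits.
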(event `self.ReceiveBeginPlay`
  (bind _asbp_pawn_truck (cast `/Game/GGJ2020Project/Blueprints/BP_Pawn_Truck` (`GameplayStatics.GetPlayerPawn` 0)))
  (set `self.PlayerPawn` _asbp_pawn_truck)
  (`AudioComponent.Play` (`self.Audio`) 0.0)
  (bind _returnvalue (`|CreateWidget` "/Game/GGJ2020Project/Widgets/WB_Main.WB_Main_C"))
  (bind _output_get (set `self.WB_Main` _returnvalue))
  (bind _output_get_2 (set `/Game/GGJ2020Project/Blueprints/BP_Pawn_Truck.WB_Main` _output_get (`self.PlayerPawn`)))
  (`UserWidget.AddToViewport` _output_get_2 0)
  (`KismetSystemLibrary.ExecuteConsoleCommand` "viewmode unlit" null)
  (`WidgetBlueprintLibrary.SetInputMode_GameOnly` self)
  (set `self.bShowMouseCursor` false))

(event `InputAction|MoveMenu`
  (params (Key :type "Key Structure"))
  (bind _wb_main (`self.WB_Main`))
  (bind _wb_credits (`/Game/GGJ2020Project/Widgets/WB_Main.WB_Credits` _wb_main))
  (:`Pressed`
    (if (`Widget.IsVisible` (`/Game/GGJ2020Project/Widgets/WB_Main.WB_GameOver` (`self.WB_Main`)))
      (`/Game/GGJ2020Project/Widgets/WB_GameOver.TriggerSpawnOut` (`/Game/GGJ2020Project/Widgets/WB_Main.WB_GameOver` _wb_main))
      (`Widget.SetVisibility` _wb_credits "Visible")
      (`/Game/GGJ2020Project/Widgets/WB_Credits.TriggerScroll` _wb_credits))))

(fn `GameOver`
  (bind _wb_main (`self.WB_Main`))
  (bind _wb_gameover (`/Game/GGJ2020Project/Widgets/WB_Main.WB_GameOver` (`self.WB_Main`)))
  (if (not (`Widget.IsVisible` _wb_gameover))
    (`Widget.SetVisibility` _wb_gameover "Visible")
    (`TextBlock.SetText` (`/Game/GGJ2020Project/Widgets/WB_GameOver.ScoreText` _wb_gameover) (`|FormatText` "YOUR FINAL SCORE IS: \n{Score} pts \nPRESS \"X\" TO CONTINUE" (`KismetTextLibrary.Conv_IntToText` (`/Game/GGJ2020Project/Blueprints/BP_Pawn_Truck.Score` (`self.PlayerPawn`)) false false)))
    (bind _outactors (`GameplayStatics.GetAllActorsOfClass` "/Game/GGJ2020Project/Blueprints/BP_Pawn_Car.BP_Pawn_Car_C"))
    (for _array_element _outactors
      (set `/Game/GGJ2020Project/Blueprints/BP_Pawn_Car.Speed` 0.0 _array_element))
    (bind _outactors_2 (`GameplayStatics.GetAllActorsOfClass` "/Game/GGJ2020Project/Blueprints/BP_Actor_Pothole.BP_Actor_Pothole_C"))
    (for _array_element_2 _outactors_2
      (set `/Game/GGJ2020Project/Blueprints/BP_Actor_Pothole.Speed` 0.0 _array_element_2))
    (bind _outactors_3 (`GameplayStatics.GetAllActorsOfClass` "/Game/GGJ2020Project/Blueprints/BP_Actor_Spawner.BP_Actor_Spawner_C"))
    (for _array_element_3 _outactors_3
      (`self.K2_DestroyActor` _array_element_3))
    (`KismetMaterialLibrary.SetScalarParameterValue` "/Game/GGJ2020Project/Materials/MPC_Background.MPC_Background" "Speed1")
    (`self.DisableInput` (cast `/Game/GGJ2020Project/Blueprints/BP_Pawn_Truck` (`GameplayStatics.GetPlayerPawn` 0) :!pure true) self)
    (`AudioComponent.SetSound` (`self.Audio`) "/Game/GGJ2020Project/Sounds/SW_Coqui.SW_Coqui")
    (`/Game/GGJ2020Project/Widgets/WB_GameOver.TriggerSpawnIn` (`/Game/GGJ2020Project/Widgets/WB_Main.WB_GameOver` _wb_main))
    (`/Game/GGJ2020Project/Widgets/WB_Main.TriggerSpawnOut` _wb_main)))

(fn `UserConstructionScript`)