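; BP_Actor_Spawner repeatedly spawns road traffic and hazards at its own transform: cars, pickup trucks, a motorcycle, a tank and potholes.
; BeginPlay starts a looping timer with an interval randomized once between MinTime and MaxTime, so each spawner keeps a fixed rhythm.
; Each tick of that timer picks a class by random index between MinIndex and MaxIndex and always spawns it, ignoring collision.
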(event `self.ReceiveBeginPlay`
  (`KismetSystemLibrary.K2_SetTimerDelegate` (delegate `SpawnActor`) (`KismetMathLibrary.RandomFloatInRange` (`self.MinTime`) (`self.MaxTime`)) true))

(event `SpawnActor`
  (`|SpawnActorFromClass` (select `int` (`KismetMathLibrary.RandomIntegerInRange` (`self.MinIndex`) (`self.MaxIndex`)) :`0` "/Game/GGJ2020Project/Blueprints/BP_Pawn_Car_Red.BP_Pawn_Car_Red_C" :`1` "/Game/GGJ2020Project/Blueprints/BP_Pawn_Car_Blue.BP_Pawn_Car_Blue_C" :`2` "/Game/GGJ2020Project/Blueprints/BP_Pawn_Car_Purple.BP_Pawn_Car_Purple_C" :`3` "/Game/GGJ2020Project/Blueprints/BP_Actor_Pothole.BP_Actor_Pothole_C" :`4` "/Game/GGJ2020Project/Blueprints/BP_Actor_Pothole_Big.BP_Actor_Pothole_Big_C" :`5` "/Game/GGJ2020Project/Blueprints/BP_Pawn_PickupTruck.BP_Pawn_PickupTruck_C" :`6` "/Game/GGJ2020Project/Blueprints/BP_Pawn_PickupTruck_Yellow.BP_Pawn_PickupTruck_Yellow_C" :`7` "/Game/GGJ2020Project/Blueprints/BP_Pawn_Motorcycle.BP_Pawn_Motorcycle_C" :`8` "/Game/GGJ2020Project/Blueprints/BP_Pawn_Tank.BP_Pawn_Tank_C" :!type "Actor Class Reference") (`self.GetTransform`) "AlwaysSpawn" "OverrideRootScale" null null))

(fn `UserConstructionScript`)