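; BP_Actor_Projectile is an asphalt shot that patches potholes for score and plays a random firing sound on spawn.
; Its box overlap casts to pothole, car or spawner to pick the response.
; Potholes switch to an asphalt sprite and award their score once via PlayerPawn, disabling collision.
; Hit cars cost score, slow down and curse; scored hits and spawner contact destroy the projectile.
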(event `self.ReceiveBeginPlay`
  (`GameplayStatics.PlaySoundAtLocation` (select `int` (`KismetMathLibrary.RandomInteger` 3) :`0` "/Game/GGJ2020Project/Sounds/SW_Shoot_01.SW_Shoot_01" :`1` "/Game/GGJ2020Project/Sounds/SW_Shoot_02.SW_Shoot_02" :`2` "/Game/GGJ2020Project/Sounds/SW_Shoot_03.SW_Shoot_03" :!type "SoundBase Object Reference") (`self.K2_GetActorLocation`) (struct) 5.0 1.0 0.0 null null null))

(event `self.Box.OnComponentBeginOverlap`
  (params (OverlappedComponent :type "PrimitiveComponent Object Reference") (OtherActor :type "Actor Object Reference") (OtherComp :type "PrimitiveComponent Object Reference") (OtherBodyIndex :type Integer) (bFromSweep :type Boolean) (SweepResult :type "HitResult Structure (by ref)"))
  (bind _asbp_actor_pothole (cast `/Game/GGJ2020Project/Blueprints/BP_Actor_Pothole` OtherActor)
    (:`then`
      (bind (_returnvalue_x _returnvalue_y) (`KismetMathLibrary.BreakVector` (`self.K2_GetActorLocation` _asbp_actor_pothole)))
      (`self.K2_SetActorLocation` _asbp_actor_pothole (`KismetMathLibrary.MakeVector` _returnvalue_x _returnvalue_y -8.0) false false)
      (`PaperSpriteComponent.SetSprite` (`/Game/GGJ2020Project/Blueprints/BP_Actor_Pothole.PaperSprite` _asbp_actor_pothole) "/Game/GGJ2020Project/Sprites/Sprite_Asphalt.Sprite_Asphalt")
      (bind _playerpawn (`self.PlayerPawn`)
        (:`then`
          (bind _box (`/Game/GGJ2020Project/Blueprints/BP_Actor_Pothole.Box` _asbp_actor_pothole))
          (if (`PrimitiveComponent.K2_IsCollisionEnabled` _box)
            (`/Game/GGJ2020Project/Blueprints/BP_Pawn_Truck.UpdateScore` _playerpawn (`/Game/GGJ2020Project/Blueprints/BP_Actor_Pothole.Score` _asbp_actor_pothole))
            (`PrimitiveComponent.SetCollisionEnabled` _box "NoCollision")
            (`GameplayStatics.PlaySoundAtLocation` "/Game/GGJ2020Project/Sounds/SW_AsphaltSplat.SW_AsphaltSplat" (`self.K2_GetActorLocation`) (struct) 5.0 (`KismetMathLibrary.RandomFloatInRange` 1.0 2.0) 0.0 null null null)
            (`self.K2_DestroyActor`)))
        (:`else`)))
    (:`CastFailed`
      (bind _asbp_pawn_car (cast `/Game/GGJ2020Project/Blueprints/BP_Pawn_Car` OtherActor)
        (:`then`
          (bind _playerpawn_2 (`self.PlayerPawn`)
            (:`then`
              (`/Engine/EditorBlueprintResources/StandardMacros.DoOnce` false
                (:`Completed`
                  (`/Game/GGJ2020Project/Blueprints/BP_Pawn_Truck.UpdateScore` _playerpawn_2 -200)
                  (`/Game/GGJ2020Project/Blueprints/BP_Pawn_Car.DecreaseSpeed` _asbp_pawn_car)
                  (`GameplayStatics.PlaySoundAtLocation` "/Game/GGJ2020Project/Sounds/SW_CursingGibberish.SW_CursingGibberish" (`self.K2_GetActorLocation` _asbp_pawn_car) (struct) 3.0 (`KismetMathLibrary.RandomFloatInRange` 1.0 1.5) 0.0 null null null)
                  (`self.K2_DestroyActor`))))
            (:`else`)))
        (:`CastFailed`
          (cast `/Game/GGJ2020Project/Blueprints/BP_Actor_Spawner` OtherActor)
          (`self.K2_DestroyActor`))))))

(fn `UserConstructionScript`)